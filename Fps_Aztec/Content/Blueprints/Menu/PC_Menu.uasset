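; PC_Menu is the main menu player controller, handling multiplayer session hosting, searching and joining.
; BeginPlay creates the WG_Menu widget once and shows the cursor with Game-and-UI input.
; Heberger creates an online session, then opens FirstPersonMap as a listen server; Rechercher fills the menu's list with a WG_Session widget per found session.
; Joining uses either a search result via JoinSession or an IP through an "open" console command in Rejoindre.
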(event Custom|Hud_Menu
  ;[0.04004 0.4271 0.0619] HUD
  (Utilities|IsValid (Variables|Default|GetHUD%20Menu)
    (:Is%20Not%20Valid
      (bind _returnvalue (UserInterface|CreateWidget "/Game/Widget/WG_Menu.WG_Menu_C"))
      (bind _output_get (Variables|Default|SetHUD%20Menu _returnvalue))
      (UserInterface|Viewport|AddtoViewport _output_get 0))))

(event Custom|Heberger
  ;[0.1823 0 0] Creer une session
  (|Session self 4 false
    (:OnSuccess
      (Game|OpenLevel(byObjectReference) "/Game/FirstPerson/Maps/FirstPersonMap.FirstPersonMap" true "listen"))))

(event Custom|Rejoindre
  (params (IP :type String))
  ;[1 0.8355 0] Rejoindre
  (Development|ExecuteConsoleCommand (Utilities|String|Append "open " IP) 0))

(event Custom|Rechercher
  ;[0 0.945 1] Rechercher
  (Widget|Panel|ClearChildren (Variables|/Game/Widget/WG_Menu.WG_Menu_C|GetVB_List_Session (Variables|Default|GetHUD%20Menu)))
  (bind _results (|FindSessions self 10 false)
    (:OnSuccess
      (Variables|Default|SetIsFindingSessions true)
      (for _array_element _results
        (bind _returnvalue (UserInterface|CreateWidget "/Game/Widget/WG_Session.WG_Session_C" 0 _array_element))
        (Widget|Panel|AddChild (Variables|/Game/Widget/WG_Menu.WG_Menu_C|GetVB_List_Session (Variables|Default|GetHUD%20Menu)) _returnvalue))
      (Variables|Default|SetIsFindingSessions false))))

(event Custom|Join%20Session
  (params (SearchResult :type Blueprint%20Session%20Result%20Structure%20%28by%20ref%29))
  ;[1 0.1156 0.5873] Join Session
  (|JoinSession self SearchResult))

(event EventBeginPlay
  ;[0.04004 0.4271 0.0619] HUD
  (CallFunction|HudMenu)
  (Variables|Default|SetbShowMouseCursor true)
  (Input|SetInputModeGameandUI self 0 "LockAlways" false false))

(fn ConstructionScript)